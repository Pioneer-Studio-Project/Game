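; BP_CeilingLight_2 is a modern ceiling light prop for the HostClub assets, with eight point lights and a Lit toggle.
; All setup runs in the construction script; the event graph is empty.
; When Lit, it applies the exposed intensity, indirect intensity, radius and temperature to the lights and swaps the mesh to the lit material.
; When unlit, it zeroes only the attenuation radius and restores the standard material.
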(fn `UserConstructionScript`
  (bind _sm_ceilinglight_modern (`self.SM_CeilingLight_Modern`))
  (bind _array (`|MakeArray` (`self.PointLight`) (`self.PointLight1`) (`self.PointLight2`) (`self.PointLight3`) (`self.PointLight4`) (`self.PointLight5`) (`self.PointLight6`) (`self.PointLight7`)))
  (if (`self.Lit`)
    (for _array_element _array
      (`LightComponent.SetIndirectLightingIntensity` _array_element (`self.Indirect Intensity`))
      (`LocalLightComponent.SetAttenuationRadius` _array_element (`self.Radius`))
      (`LightComponent.SetIntensity` _array_element (`self.Intensity`))
      (`LightComponent.SetTemperature` _array (`self.Temperature`))
      (`PrimitiveComponent.SetMaterial` _sm_ceilinglight_modern 0 "/Game/Assets/HostClub/Assets/Props/Materials/MI_Lit.MI_Lit"))
    (else
      (for _array_element_2 _array
        (`LocalLightComponent.SetAttenuationRadius` _array_element_2 0.0)
        (`LocalLightComponent.SetAttenuationRadius` _array_element_2 0.0)
        (`PrimitiveComponent.SetMaterial` _sm_ceilinglight_modern 0 "/Game/Assets/HostClub/Assets/Props/Materials/MI_CeilingLight_Modern.MI_CeilingLight_Modern")))))